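; Main menu game mode that shows the mouse cursor on BeginPlay and opens the main menu widget.
; SwitchWidget clears all widgets, then creates and displays the main menu, character selection or game settings widget based on its parameter.
; Main menu and settings use UI-only input without mouse lock, while character selection uses Game and UI input focused on its widget.
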(event `self.ReceiveBeginPlay`
  (set `PlayerController.bShowMouseCursor` true (`GameplayStatics.GetPlayerController` 0))
  (`self.SwitchWidget` "NewEnumerator0"))

(fn `SwitchWidget`
  (params (NewParam :type "/Game/UI/MainMenu/Enum_MainMenuWidget Enum" :default "NewEnumerator0"))
  (`WidgetLayoutLibrary.RemoveAllWidgets`)
  (switch `/Game/UI/MainMenu/Enum_MainMenuWidget` NewParam
    (:`NewEnumerator0`
      (bind _returnvalue (`|CreateWidget` "/Game/UI/MainMenu/WBP_MainMenu.WBP_MainMenu_C"))
      (`UserWidget.AddToViewport` _returnvalue 0)
      (`WidgetBlueprintLibrary.SetInputMode_UIOnlyEx` (`GameplayStatics.GetPlayerController` 0) null))
    (:`NewEnumerator1`
      (bind _returnvalue_2 (`|CreateWidget` "/Game/UI/MainMenu/WBP_PlayerSelection.WBP_PlayerSelection_C"))
      (`UserWidget.AddToViewport` _returnvalue_2 0)
      (`WidgetBlueprintLibrary.SetInputMode_GameAndUIEx` (`GameplayStatics.GetPlayerController` 0) _returnvalue_2))
    (:`NewEnumerator2`
      (bind _returnvalue_3 (`|CreateWidget` "/Game/UI/MainMenu/WBP_GameSettings.WBP_GameSettings_C"))
      (`UserWidget.AddToViewport` _returnvalue_3 0)
      (`WidgetBlueprintLibrary.SetInputMode_UIOnlyEx` (`GameplayStatics.GetPlayerController` 0) null))))

(fn `UserConstructionScript`)