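; BP_PlayerSelection is the character selection actor that previews the playable characters before the Bomberman match starts.
; Left and right inputs step a wrapping index through parallel skeletal mesh and anim class arrays, starting from the first entry.
; Each change updates the previewed mesh and animation and passes both to BP_BombermanGameInstance through UpdateMesh.
; The SpawnBomb input doubles as confirm and opens GameLevel.
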(event `self.ReceiveBeginPlay`
  ;[1 1 1] Set the default mesh of the player
  (set `self.playerMeshIndex` 0)
  (`self.ChangePlayerMesh`))

(event `InputAction|SelectLeft`
  (params (Key :type "Key Structure"))
  (:`Pressed`
    (bind _output_get (set `self.playerMeshIndex` (+ (`self.playerMeshIndex`) -1)))
    (if (< _output_get 0)
      (set `self.playerMeshIndex` (- (`KismetArrayLibrary.Array_Length` (`self.PlayerMesh`)) 1)))
    (`self.ChangePlayerMesh` :!label _label)))

(event `InputAction|SelectRight`
  (params (Key :type "Key Structure"))
  (:`Pressed`
    (if true
      (bind _output_get (set `self.playerMeshIndex` (+ (`self.playerMeshIndex`) 1)))
      (if (> _output_get (- (`KismetArrayLibrary.Array_Length` (`self.PlayerMesh`)) 1))
        (set `self.playerMeshIndex` 0)
        (goto _label)
        (else
          (goto _label))))))

(event `InputAction|SpawnBomb`
  (params (Key :type "Key Structure"))
  (:`Pressed`
    (`GameplayStatics.OpenLevel` "GameLevel")))

(fn `ChangePlayerMesh`
  (bind _output (`|GetArrayItem` (`self.PlayerMesh`) (`self.playerMeshIndex`)))
  (bind _output_2 (`|GetArrayItem` (`self.playerAnim`) (`self.playerMeshIndex`)))
  (`SkinnedMeshComponent.SetSkinnedAssetAndUpdate` (`self.SkeletalMesh`) _output true)
  (`SkeletalMeshComponent.SetAnimInstanceClass` (`self.SkeletalMesh`) _output_2)
  (bind _asbp_bomberman_game_instance (cast `/Game/GameSettings/BP_BombermanGameInstance` (`GameplayStatics.GetGameInstance`)))
  (`/Game/GameSettings/BP_BombermanGameInstance.Update Mesh` _asbp_bomberman_game_instance _output _output_2))

(fn `UserConstructionScript`)