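; Base player character Blueprint that handles movement along fixed world axes and turns the mesh to face the input direction.
; MoveForward feeds movement input along world X and MoveRight along world Y, independent of camera or control rotation.
; The sign of each nonzero axis value snaps the Mesh to one of four cardinal world yaws, with no interpolation or diagonal facing.
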(event `InputAxis|MoveForward`
  (params (AxisValue :type "Float (single-precision)"))
  (bind _mesh (`self.Mesh`))
  (if (< AxisValue 0.0)
    (`SceneComponent.K2_SetWorldRotation` _mesh (struct :`Yaw` 90.0) false false)
    (`self.AddMovementInput` (1.0 0.0 0.0) AxisValue :!label _label)
    (elif (> AxisValue 0.0)
      (`SceneComponent.K2_SetWorldRotation` _mesh (struct :`Yaw` 270.0) false false)
      (goto _label))))

(event `InputAxis|MoveRight`
  (params (AxisValue :type "Float (single-precision)"))
  (bind _mesh (`self.Mesh`))
  (if (< AxisValue 0.0)
    (`SceneComponent.K2_SetWorldRotation` _mesh (struct :`Yaw` 180.0) false false)
    (`self.AddMovementInput` (0.0 1.0 0.0) AxisValue :!label _label_2)
    (elif (> AxisValue 0.0)
      (`SceneComponent.K2_SetWorldRotation` _mesh (struct) false false)
      (goto _label_2))))

(fn `UserConstructionScript`)